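; BP_Amb_Pipe_Spline is a soundscape actor that slides a looping water sound along a spline to follow the player.
; A looping timer started at BeginPlay finds the spline point closest to the player every 0.05 seconds.
; The audio's position lerps toward that point using the SmoothMoving timeline's value.
; Larger X or Y jumps trigger the timeline through a DoOnce, which resets when playback finishes.
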(event Custom|Move_Audio
  (bind _spline (Variables|Default|GetSpline))
  (bind _player_char_ref (Variables|Default|GetPlayer_Char_Ref))
  (bind _returnvalue (Transformation|GetActorLocation _player_char_ref))
  (bind _returnvalue_2 (Spline|FindLocationClosesttoWorldLocation _spline _returnvalue "World"))
  (if (not (or (> (Math|Float|Absolute(Float) (.x (- (Spline|FindLocationClosesttoWorldLocation (Variables|Default|GetSpline) (Transformation|GetActorLocation (Variables|Default|GetPlayer_Char_Ref)) "World") (Variables|Default|GetPrevious_Loc)))) 1e+01) (> (Math|Float|Absolute(Float) (.y (- (Spline|FindLocationClosesttoWorldLocation (Variables|Default|GetSpline) (Transformation|GetActorLocation (Variables|Default|GetPlayer_Char_Ref)) "World") (Variables|Default|GetPrevious_Loc)))) 1e+01)))
    (Transformation|SetWorldLocation (Variables|Default|GetWaterLp) (Math|Vector|Lerp(Vector) (Variables|Default|GetPrevious_Loc) _returnvalue_2 (stale _float)) false false :!label _label)
    (Variables|Default|SetPrevious_Loc _returnvalue_2)
    (else
      (Utilities|FlowControl|DoOnce false :!label _label_2
        (:Completed
          (Variables|Default|SetisTransitioning true)
          ;[1 0 0] need to toggle this
          (if (Variables|Default|GetisTransitioning)
            (bind _float (Timeline|SmoothMoving Play)
              (:Update
                (goto _label))
              (:Finished
                (Variables|Default|SetisTransitioning false)
                (goto _label_2 Reset)))))))))

(event EventBeginPlay
  (bind _returnvalue (Actor|GetActorOfClass "/Script/Malignant.PlayerCharacter"))
  (Variables|Default|SetPlayer_Char_Ref _returnvalue)
  (if (not (Utilities|Time|IsTimerActivebyHandle (Variables|Default|GetTmr_Move_Audio)))
    (bind _returnvalue_2 (Utilities|Time|SetTimerbyEvent (delegate Custom|Move_Audio) 0.05 true))
    (Variables|Default|SetTmr_Move_Audio _returnvalue_2)))

(fn ConstructionScript)