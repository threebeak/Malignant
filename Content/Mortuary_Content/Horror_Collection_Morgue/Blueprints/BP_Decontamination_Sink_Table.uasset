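; Decontamination sink table prop for a morgue set, with four doors whose opening angles are set through per-door variables.
; The construction script passes each variable to a RotateZ helper that sets that door mesh's relative yaw, negating it for the third and fourth doors.
; The event graph holds only disabled stub events, so the asset has no runtime door logic.
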(event EventBeginPlay)

(event Collision|EventActorBeginOverlap
  (params (OtherActor :type Actor%20Object%20Reference)))

(event EventTick
  (params (DeltaSeconds :type Float%20%28single-precision%29)))

(fn ConstructionScript
  (CallFunction|RotateZ (Variables|Doors|GetOpenDoor_1st) false (Variables|Default|GetSM_Sink_Door1))
  (CallFunction|RotateZ (Variables|Doors|GetOpenDoor_2nd) false (Variables|Default|GetSM_Sink_Door2))
  (CallFunction|RotateZ (Variables|Doors|GetOpenDoor_3rd) true (Variables|Default|GetSM_Sink_Door3))
  (CallFunction|RotateZ (Variables|Doors|GetOpenDoor_4th) true (Variables|Default|GetSM_Sink_Door4)))

(fn RotateZ
  (params (Z%20%28Yaw%29 :type Float%20%28double-precision%29) (InvertZ :type Boolean) (TargetMesh :type Scene%20Component%20Object%20Reference))
  (if InvertZ
    (Transformation|SetRelativeRotation TargetMesh (Math|Rotator|MakeRotator 0.0 0.0 (* Z%20%28Yaw%29 -1.0)) false false)
    (else
      (Transformation|SetRelativeRotation TargetMesh (Math|Rotator|MakeRotator 0.0 0.0 Z%20%28Yaw%29) false false)))
  (return))