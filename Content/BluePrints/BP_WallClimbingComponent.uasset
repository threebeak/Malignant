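; BP_WallClimbingComponent is an actor component that toggles wall climbing on the player character.
; On BeginPlay it caches the owning PlayerCharacter.
; StartWallClimb and StopWallClimb switch the character movement between a Custom mode and Falling, guarded by an IsClimbing flag.
; The component contains no wall detection or climbing movement logic of its own.
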(event Custom|StartWallClimb
  (bind _player (Variables|Default|GetPlayer))
  (if (not (Variables|Default|GetIsClimbing))
    (Utilities|IsValid _player
      (:Is%20Valid
        (Pawn|Components|CharacterMovement|SetMovementMode (Variables|/Script/Engine.Character|GetCharacterMovement _player) "MOVE_Custom" 0)
        (Variables|Default|SetIsClimbing true)))))

(event Custom|StopWallClimb
  (if (Variables|Default|GetIsClimbing)
    (Pawn|Components|CharacterMovement|SetMovementMode (Variables|/Script/Engine.Character|GetCharacterMovement (Variables|Default|GetPlayer)) "MOVE_Falling" 0)
    (Variables|Default|SetIsClimbing false)))

(event EventBeginPlay
  (bind _asplayer_character (Utilities|Casting|CastToPlayerCharacter (Components|GetOwner)))
  (Variables|Default|SetPlayer _asplayer_character))

(event EventTick
  (params (DeltaSeconds :type Float%20%28single-precision%29)))