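; Desk Blueprint from the repair system: a desk the player can pick up and carry at reduced walk speed.
; TakeDesk and Interact share a DoOnce that registers the desk as the LastStandCharacter's held table, sets the carry flags and lowers MaxWalkSpeed.
; ResetTakeDesk re-arms the DoOnce for another pickup; attaching the desk and restoring speed are not handled here.
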(event Custom|ResetTakeDesk
  (Utilities|FlowControl|DoOnce false) ; enters at Reset
)

(event Custom|TakeDesk
  (Utilities|FlowControl|DoOnce false
    (:Completed
      (bind _aslast_stand_character (Utilities|Casting|CastToLastStandCharacter (Game|GetPlayerCharacter 0)))
      (Variables|/Game/Levels/LastStandCharacter.LastStandCharacter_C|SetHeldTable _aslast_stand_character self)
      (Variables|/Game/Levels/LastStandCharacter.LastStandCharacter_C|SetIsObjectTacked _aslast_stand_character true)
      (Variables|Default|SetIsDesk true)
      (Variables|/Script/Engine.CharacterMovementComponent|SetMaxWalkSpeed (Variables|/Script/Engine.Character|GetCharacterMovement (Game|GetPlayerCharacter 0)) 1.5e+02))))

(event EventInteract
  (Utilities|FlowControl|DoOnce false
    (:Completed
      (bind _aslast_stand_character (Utilities|Casting|CastToLastStandCharacter (Game|GetPlayerCharacter 0)))
      (Variables|/Game/Levels/LastStandCharacter.LastStandCharacter_C|SetHeldTable _aslast_stand_character self)
      (Variables|/Game/Levels/LastStandCharacter.LastStandCharacter_C|SetIsObjectTacked _aslast_stand_character true)
      (Variables|Default|SetIsDesk true)
      (Variables|/Script/Engine.CharacterMovementComponent|SetMaxWalkSpeed (Variables|/Script/Engine.Character|GetCharacterMovement (Game|GetPlayerCharacter 0)) 1.5e+02))))

(fn ConstructionScript)