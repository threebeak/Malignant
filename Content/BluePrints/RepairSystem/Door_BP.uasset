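; Repairable door that gains health from a carried chair and shows its health in a widget while the player overlaps its Box.
; Tick polls the R key and the first Chair_BP's TakeChair flag, without checking overlap.
; A never-reset DoOnce then adds the chair's health, restores walk speed and clears the flag.
; Tick also pushes Health into the first on-screen W_DoorHealth found by class search.
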(event OnComponentBeginOverlap(Box)
  (params (OverlappedComponent :type Primitive%20Component%20Object%20Reference) (OtherActor :type Actor%20Object%20Reference) (OtherComp :type Primitive%20Component%20Object%20Reference) (OtherBodyIndex :type Integer) (bFromSweep :type Boolean) (SweepResult :type Hit%20Result%20Structure%20%28by%20ref%29))
  (Utilities|Casting|CastToPlayerCharacter OtherActor)
  (bind _returnvalue (UserInterface|CreateWidget "/Game/BluePrints/RepairSystem/W_DoorHealth.W_DoorHealth_C"))
  (UserInterface|Viewport|AddtoViewport _returnvalue 0))

(event OnComponentEndOverlap(Box)
  (params (OverlappedComponent :type Primitive%20Component%20Object%20Reference) (OtherActor :type Actor%20Object%20Reference) (OtherComp :type Primitive%20Component%20Object%20Reference) (OtherBodyIndex :type Integer))
  (Utilities|Casting|CastToPlayerCharacter OtherActor)
  (Widget|RemovefromParent (stale OnComponentBeginOverlap(Box) _returnvalue)))

(event EventBeginPlay
  (Utilities|FlowControl|Sequence
    (:then_0
      (bind _outactors (Actor|GetAllActorsOfClass "/Game/BluePrints/RepairSystem/Chair_BP.Chair_BP_C"))
      (Variables|Default|SetChairs (Utilities|Array|Get(acopy) _outactors)))))

(event EventTick
  (params (DeltaSeconds :type Float%20%28single-precision%29))
  (bind _chairs (Variables|Default|GetChairs))
  (Utilities|FlowControl|Sequence
    (:then_0
      (Utilities|FlowControl|Delay 0.1)
      (if (and (Game|Player|IsInputKeyDown (Game|GetPlayerController 0) "R") (Variables|/Game/BluePrints/RepairSystem/Chair_BP.Chair_BP_C|GetTakeChair _chairs))
        (Utilities|FlowControl|DoOnce false
          (:Completed
            (Variables|Default|SetHealth (+ (Variables|/Game/BluePrints/RepairSystem/Chair_BP.Chair_BP_C|GetHealth _chairs) (Variables|Default|GetHealth)))
            (Variables|/Script/Engine.CharacterMovementComponent|SetMaxWalkSpeed (Variables|/Script/Engine.Character|GetCharacterMovement (Game|GetPlayerCharacter 0)) 6e+02)
            (Variables|/Game/BluePrints/RepairSystem/Chair_BP.Chair_BP_C|SetTakeChair _chairs false)
            (Development|PrintString (Utilities|String|ToString(Float) (Variables|Default|GetHealth)))))))
    (:then_1
      (bind _foundwidgets (Widget|GetAllWidgetsOfClass "/Game/BluePrints/RepairSystem/W_DoorHealth.W_DoorHealth_C" true))
      (bind _asw_door_health (Utilities|Casting|CastToW_DoorHealth (Utilities|Array|Get(acopy) _foundwidgets)))
      (Variables|/Game/BluePrints/RepairSystem/W_DoorHealth.W_DoorHealth_C|SetDoorsHealth _asw_door_health (Variables|Default|GetHealth)))))

(fn ConstructionScript)