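; Playable BoneBlade mutant character with melee blade attacks, three abilities, item equipping and separate first- and third-person meshes.
; Attacks run a looping timer that line-traces between both blades' sockets to damage test dummies.
; Abilities fire bone projectiles through a component, call a print-only SharpenBones stub, or charge an AOE while slowing movement.
; On release, a timeline grows a debug-drawn sphere that collects and prints overlapped enemies without damaging them.
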(event Custom|BoneAOE
  (bind _overlapping_actors (Variables|Default|GetOverlapping%20Actors))
  (if (not (Variables|Default|GetAOETriggered))
    (Variables|Default|SetAOETriggered true)
    (bind _returnvalue (AddComponent|AddSphereComponent false))
    (bind _newtrack_0 (Timeline|SphereTrace PlayFromStart)
      (:Update
        (Transformation|SetWorldScale3D _returnvalue (Math|Vector|Lerp(Vector) "0, 0, 0" (Variables|Default|GetAOE%20Radius) _newtrack_0))
        (Rendering|Debug|DrawDebugSphere (Transformation|GetActorLocation) (Components|Sphere|GetScaledSphereRadius _returnvalue) 12 "(R=0.030518,G=1.000000,B=0.000000,A=1.000000)" 0.1 0.5)
        (for _array_element (Collision|GetOverlappingActors _returnvalue "/Script/Malignant.BaseEnemy" :!class /Script/Engine.PrimitiveComponent)
          (Utilities|Set|Add (Variables|Default|GetOverlapping%20Actors) _array_element)))
      (:Finished
        (Components|DestroyComponent _returnvalue)
        (if (Utilities|Set|IsEmpty _overlapping_actors)
          _
          (else
            (bind _result (Utilities|Set|ToArray _overlapping_actors))
            (for _array_element_2 _result
              (Development|PrintString (Utilities|GetDisplayName _array_element_2)))
            (Utilities|Set|Clear (Variables|Default|GetOverlapping%20Actors))))
        (Variables|Default|SetAOE%20Radius "0, 0, 0")
        (Variables|Default|SetAOETriggered false)
        (Development|PrintString "Reset")))))

(event Custom|AttackStart
  (CallFunction|AttackTrace)
  (bind _returnvalue (Utilities|Time|SetTimerbyFunctionName 0 "AttackTrace" 0.01 true))
  (Variables|Default|SetAttackHandle _returnvalue))

(event Custom|AttackEnd
  (Utilities|Time|ClearandInvalidateTimerbyHandle (Variables|Default|GetAttackHandle)))

(event Custom|setCharacterVisibility
  (bind _meshbodyfps (Variables|Default|GetMeshBodyFPS))
  ;[1 1 1] set character visibility
  (Rendering|SetOnlyOwnerSee (Variables|Character|GetMesh) true :!class /Script/Engine.PrimitiveComponent)
  (Class|PrimitiveComponent|SetOwnerNoSee (Variables|Default|GetMeshTPS) true)
  (Rendering|SetOnlyOwnerSee _meshbodyfps true :!class /Script/Engine.PrimitiveComponent)
  (Components|SkinnedMesh|HideBonebyName _meshbodyfps "l_bicep" "PBO_None")
  (Components|SkinnedMesh|HideBonebyName _meshbodyfps "r_bicep" "PBO_None")
  (Components|SkinnedMesh|HideBonebyName _meshbodyfps "neck" "PBO_None"))

(event EventBeginPlay
  (CallFunction|SetCharacterVisibility))

(event Collision|EventActorBeginOverlap
  (params (OtherActor :type Actor%20Object%20Reference)))

(event EventTick
  (params (DeltaSeconds :type Float%20%28single-precision%29)))

(event EventEquipItem
  (params (NewItem :type Object%20Object%20Reference))
  (Utilities|IsValid NewItem
    (:Is%20Valid
      (Variables|Default|SetEquippedItem NewItem)
      (Collision|SetActorEnableCollision NewItem false)
      (Transformation|AttachComponentToComponent NewItem (Variables|Character|GetMesh) "R_HandSocket" "SnapToTarget" "KeepRelative" "KeepWorld" false))))

(event Input|ActionEvents|InputActionAbility1
  (params (Key :type Key%20Structure :default "None"))
  (:Pressed
    (Default|FireBone (Variables|Default|GetBP_BoneProjectileComponent))))

(event Input|ActionEvents|InputActionAbility2
  (params (Key :type Key%20Structure :default "None"))
  (:Pressed
    (CallFunction|SharpenBones)))

(event Input|ActionEvents|InputActionAbility3
  (params (Key :type Key%20Structure :default "None"))
  (:Pressed
    (if (not (Variables|Default|GetAOETriggered))
      (Variables|/Script/Engine.CharacterMovementComponent|SetMaxWalkSpeed (Variables|Character|GetCharacterMovement) 5e+01)
      (bind _returnvalue (Utilities|Time|SetTimerbyFunctionName 0 "AddCharge" 0.2 true))
      (Variables|Default|SetAOEChargeHandle _returnvalue)))
  (:Released
    (Variables|/Script/Engine.CharacterMovementComponent|SetMaxWalkSpeed (Variables|Character|GetCharacterMovement) 6e+02)
    (Utilities|Time|ClearandInvalidateTimerbyHandle (Variables|Default|GetAOEChargeHandle))
    (if (> (Variables|Default|GetAOEPower) 0)
      (Variables|Default|SetAOEPower 0)
      (CallFunction|BoneAOE))))

(fn ConstructionScript)

(fn SharpenBones
  (Development|PrintString "*Shing *Shing  Damn boy now you doing hella damage "))

(fn AddCharge
  (if (< (Variables|Default|GetAOEPower) 10)
    (Math|Integer|IncrementInt (Variables|Default|GetAOEPower)
      (:%20%20
        (bind _output_get (Variables|Default|SetAOE%20Radius (+ (Variables|Default|GetAOE%20Radius) "2.000000,2.000000,2.000000")))
        (Development|PrintString (Utilities|String|ToString(Vector) _output_get))))))

(fn AttackTrace
  (bind _mesh (Variables|Character|GetMesh))
  (bind _mesh_2 (Variables|Character|GetMesh))
  (Utilities|FlowControl|Sequence
    (:then_0
      (bind _outhit (Collision|LineTraceByChannel (Transformation|GetSocketLocation _mesh_2 "R_BoneBladeSocketStart") (Transformation|GetSocketLocation _mesh_2 "R_BoneBladeSocketEnd") "TraceTypeQuery3" false 0 "ForDuration" true "(R=1.000000,G=0.000000,B=0.000000,A=1.000000)" "(R=0.000000,G=1.000000,B=0.000000,A=1.000000)" 1.0))
      (bind _asbp_test_dummy (Utilities|Casting|CastToBP_TestDummy (.HitActor (Collision|BreakHitResult _outhit))))
      (Default|OnRecieveDamage _asbp_test_dummy 1))
    (:then_1
      (bind _outhit_2 (Collision|LineTraceByChannel (Transformation|GetSocketLocation _mesh "L_BoneBladeSocketStart") (Transformation|GetSocketLocation _mesh "L_BoneBladeSocketEnd") "TraceTypeQuery3" false 0 "ForDuration" true "(R=1.000000,G=0.000000,B=0.000000,A=1.000000)" "(R=0.000000,G=1.000000,B=0.000000,A=1.000000)" 1.0))
      (bind _asbp_test_dummy_2 (Utilities|Casting|CastToBP_TestDummy (.HitActor (Collision|BreakHitResult _outhit_2))))
      (Default|OnRecieveDamage _asbp_test_dummy_2 1))))