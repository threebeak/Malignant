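; BP_Tape is a collectible music tape that the player picks up by walking into it.
; It looks up its song and tape data in DT_Tape by ID on BeginPlay and again on Tick, depending on its tape enum.
; Overlap hides the mesh and flags it taken.
; Tick then reveals the matching Metal or Classic tape and name on every cached BP_TapeStack.
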(event OnComponentBeginOverlap(Box)
  (params (OverlappedComponent :type Primitive%20Component%20Object%20Reference) (OtherActor :type Actor%20Object%20Reference) (OtherComp :type Primitive%20Component%20Object%20Reference) (OtherBodyIndex :type Integer) (bFromSweep :type Boolean) (SweepResult :type Hit%20Result%20Structure%20%28by%20ref%29))
  (Utilities|Casting|CastToPlayerCharacter OtherActor)
  (Variables|Core|SetIsTaked? true)
  (Rendering|SetVisibility (Variables|Default|GetTape) false false))

(event Custom|IDTape
  (params (ID :type Name))
  (bind _outrownames (DataTable|GetDataTableRowNames "/Game/BluePrints/Radio/DT_Tape.DT_Tape"))
  (bind _returnvalue (Utilities|GetDataTableRow "/Game/BluePrints/Radio/DT_Tape.DT_Tape" (Utilities|Array|Get(acopy) _outrownames (Utilities|Array|FindItem _outrownames ID)))
    (:then
      (Variables|Core|SetSong (.Song (Utilities|Struct|BreakST_Tape _returnvalue)))
      (Variables|Core|SetTapes (.Tape (Utilities|Struct|BreakST_Tape _returnvalue))))))

(event EventTick
  (params (DeltaSeconds :type Float%20%28single-precision%29))
  (bind _id (Variables|Editable|GetID))
  (Utilities|FlowControl|Sequence
    (:then_0
      (switch Utilities|FlowControl|Switch|SwitchonEN_Tapes (Variables|Editable|GetENTapes)
        (:NewEnumerator0
          (CallFunction|IDTape _id))
        (:NewEnumerator1
          (CallFunction|IDTape _id))))
    (:then_1
      (for _array_element (Variables|Default|GetTapeStack)
        (if (Variables|Core|GetIsTaked?)
          (if (== (Variables|Editable|GetID) "Metal")
            (Rendering|SetVisibility (Variables|/Game/BluePrints/Radio/BP_TapeStack.BP_TapeStack_C|GetTape_Metal_1 _array_element) true false)
            (elif (== (Variables|Editable|GetID) "Classic")
              (Rendering|SetVisibility (Variables|/Game/BluePrints/Radio/BP_TapeStack.BP_TapeStack_C|GetTapeName_2 _array_element) true false))))))))

(event EventBeginPlay
  (Utilities|FlowControl|Sequence
    (:then_0
      (bind _outrownames (DataTable|GetDataTableRowNames "/Game/BluePrints/Radio/DT_Tape.DT_Tape"))
      (bind _returnvalue (Utilities|GetDataTableRow "/Game/BluePrints/Radio/DT_Tape.DT_Tape" (Utilities|Array|Get(acopy) _outrownames (Utilities|Array|FindItem _outrownames (stale Custom|IDTape ID))))
        (:then
          (Variables|Core|SetSong (.Song (Utilities|Struct|BreakST_Tape _returnvalue)))
          (Variables|Core|SetTapes (.Tape (Utilities|Struct|BreakST_Tape _returnvalue))))))
    (:then_1
      (bind _outactors (Actor|GetAllActorsOfClass "/Game/BluePrints/Radio/BP_TapeStack.BP_TapeStack_C"))
      (for _array_element _outactors
        (Utilities|Array|Add (Variables|Default|GetTapeStack) _array_element)))))

(fn ConstructionScript
  (Components|StaticMesh|SetStaticMesh (Variables|Default|GetTape) (Variables|Editable|GetMesh)))