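; BP_Radio is a radio actor that plays songs from BP_Tape actors at its base's location.
; BeginPlay gathers every tape in the level, and player overlap loops over them checking IsTaked, with no action attached.
; Tick polls the Z key, without gating on overlap, to stop the current sound and spawn the next song from that loop's element.
; The song index is clamped to two entries and never wraps.
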(event OnComponentBeginOverlap(Box)
  (params (OverlappedComponent :type Primitive%20Component%20Object%20Reference) (OtherActor :type Actor%20Object%20Reference) (OtherComp :type Primitive%20Component%20Object%20Reference) (OtherBodyIndex :type Integer) (bFromSweep :type Boolean) (SweepResult :type Hit%20Result%20Structure%20%28by%20ref%29))
  (Utilities|Casting|CastToPlayerCharacter OtherActor)
  (for _array_element (Variables|Default|GetTape)
    (if (Variables|/Game/BluePrints/Radio/BP_Tape.BP_Tape_C|GetIsTaked? _array_element)
      _)))

(event EventBeginPlay
  (bind _outactors (Actor|GetAllActorsOfClass "/Game/BluePrints/Radio/BP_Tape.BP_Tape_C"))
  (for _array_element _outactors
    (Utilities|Array|Add (Variables|Default|GetTape) _array_element)))

(event EventTick
  (params (DeltaSeconds :type Float%20%28single-precision%29))
  (if (Game|Player|WasInputKeyJustPressed (Game|GetPlayerController 0) "Z")
    (Audio|Components|Audio|Stop (Variables|Default|GetCurrentSong))
    (Variables|Default|SetSelectSong (Math|Integer|Clamp(Integer) (+ (Variables|Default|GetSelectSong) 1) 0 1))
    (Development|PrintString (Utilities|String|ToString(Integer) (Variables|Default|GetSelectSong)))
    (bind _returnvalue (Audio|SpawnSoundatLocation (Utilities|Array|Get(acopy) (Variables|/Game/BluePrints/Radio/BP_Tape.BP_Tape_C|GetSong (stale OnComponentBeginOverlap(Box) _array_element)) (Variables|Default|GetSelectSong)) (Transformation|GetWorldLocation (Variables|Default|GetBase_Radio)) "0, 0, 0" 1.0 1.0 0.0 0 0))
    (Variables|Default|SetCurrentSong _returnvalue)))

(fn ConstructionScript)