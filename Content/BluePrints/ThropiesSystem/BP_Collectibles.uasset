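; BP_Collectibles is a trophy display actor that previews a collectible as a spinning mesh and fills in the W_Collectibles widget.
; A SceneCapture2D renders only this actor's components, isolating the model.
; Every Tick reapplies the hard-coded JassonMask row from DT_Collectibles: owned items set widget name and description, missing ones get a placeholder material.
; Tick also plays the Rotate timeline, which restarts on finish to loop the yaw spin.
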(event Custom|Repeat
  ;[1 1 1] Rotate Collectable
  (bind _rotate (Timeline|Rotate PlayFromStart)
    (:Update
      (Transformation|SetRelativeRotation (Variables|Default|GetTrophie_default) (Math|Rotator|MakeRotator 0.0 0.0 _rotate) false false))
    (:Finished
      (CallFunction|Repeat))))

(event Custom|ChangeMesh
  (bind _trophie_default (Variables|Default|GetTrophie_default))
  (bind _w_collectibles (Variables|Default|GetW_Collectibles))
  ;[1 1 1] Set Mesh And Text
  (bind _returnvalue (Utilities|GetDataTableRow "/Game/BluePrints/ThropiesSystem/DT_Collectibles.DT_Collectibles" "JassonMask")
    (:then
      (if (Variables|Default|GethaveTheCollectable)
        (Components|StaticMesh|SetStaticMesh (Variables|Default|GetTrophie_default) (.Mesh (Utilities|Struct|BreakST_CollectIbles _returnvalue)))
        (Rendering|Components|TextRender|SetText (Variables|/Game/BluePrints/ThropiesSystem/W_Collectibles.W_Collectibles_C|GetName _w_collectibles) (.Name (Utilities|Struct|BreakST_CollectIbles _returnvalue)))
        (Rendering|Components|TextRender|SetText (Variables|/Game/BluePrints/ThropiesSystem/W_Collectibles.W_Collectibles_C|GetDescription _w_collectibles) (.Description (Utilities|Struct|BreakST_CollectIbles _returnvalue)))
        (else
          (Components|StaticMesh|SetStaticMesh _trophie_default (.Mesh (Utilities|Struct|BreakST_CollectIbles _returnvalue)))
          (Rendering|Material|SetMaterial _trophie_default 0 "/Game/BluePrints/ThropiesSystem/M_NoHaveCollectible.M_NoHaveCollectible"))))))

(event EventBeginPlay
  ;[1 1 1] Show Only Mesh
  (Rendering|SceneCapture|ShowOnlyActorComponents (Variables|Default|GetSceneCaptureComponent2D) self false)
  (bind _foundwidgets (Widget|GetAllWidgetsOfClass "/Game/BluePrints/ThropiesSystem/W_Collectibles.W_Collectibles_C" true))
  (Variables|Default|SetW_Collectibles (Utilities|Array|Get(acopy) _foundwidgets)))

(event EventTick
  (params (DeltaSeconds :type Float%20%28single-precision%29))
  ;[1 1 1] Rotate Collectable
  (Utilities|FlowControl|Sequence
    (:then_0
      (CallFunction|ChangeMesh)
      (bind _rotate (Timeline|Rotate Play)
        (:Update
          (Transformation|SetRelativeRotation (Variables|Default|GetTrophie_default) (Math|Rotator|MakeRotator 0.0 0.0 _rotate) false false))
        (:Finished
          (CallFunction|Repeat))))))

(fn ConstructionScript)