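; BP_MalignantGameState is a game state Blueprint that swaps the player's pawn for another mutant character.
; SpawnPlayer looks up the requested CharacterClass in MutantMap, destroys player 0's current pawn and spawns the mapped actor at that pawn's location.
; The player controller then possesses the new actor, and PC_Malignant stores it as PlayerPawn.
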(event EventBeginPlay)

(event EventTick
  (params (DeltaSeconds :type Float%20%28single-precision%29)))

(event EventSpawnPlayer
  (params (CharacterClass :type EMutantState%20Enum :default "Human"))
  (bind _returnvalue (Game|Player|GetPlayerPawn 0))
  (bind _returnvalue_2 (Game|GetPlayerController 0))
  (bind _mutantmap (Variables|Default|GetMutantMap))
  (bind (_value _returnvalue_3) (Utilities|Map|Find _mutantmap CharacterClass))
  (if _returnvalue_3
    (bind _output_get (Variables|Default|SetSpawnLocation (Transformation|GetActorLocation _returnvalue)))
    (Actor|DestroyActor _returnvalue)
    (bind _returnvalue_4 (Game|SpawnActorfromClass _value (Math|Transform|MakeTransform _output_get "0, 0, 0" "1.000000,1.000000,1.000000") "Undefined" 0 0))
    (Pawn|Possess _returnvalue_2 _returnvalue_4)
    (Variables|/Game/BluePrints/PC_Malignant.PC_Malignant_C|SetPlayerPawn (.AsPC%20Malignant (Utilities|Casting|CastToPC_Malignant _returnvalue_2)) _returnvalue_4)))

(fn ConstructionScript)