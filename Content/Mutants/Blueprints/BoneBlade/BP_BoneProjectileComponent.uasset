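; Actor component for the Bone Blade mutant character that fires bone projectiles from its arm blades.
; On BeginPlay it caches the owning BP_BoneBladeMutantCharacter.
; FireBone spawns a BP_BoneProjectile with the character as instigator, aimed along the main camera's rotation.
; GetFireLocation flips a flag on each shot to alternate the spawn point between the right and left blade sockets.
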(event Custom|FireBone
  (Utilities|IsValid (Variables|Default|GetBoneBladeCharacter)
    (:Is%20Valid
      (CallFunction|GetFireLocation)
      (Game|SpawnActorfromClass "/Game/Mutants/Blueprints/BoneBlade/BP_BoneProjectile.BP_BoneProjectile_C" (Math|Transform|MakeTransform (Variables|Default|GetFireLocation) (Transformation|GetWorldRotation (Variables|/Script/Malignant.PlayerCharacter|GetMainCamera (Variables|Default|GetBoneBladeCharacter))) "1.000000,1.000000,1.000000") "Undefined" 0 (Variables|Default|GetBoneBladeCharacter)))))

(event EventBeginPlay
  (bind _asbp_bone_blade_mutant_character (Utilities|Casting|CastToBP_BoneBladeMutantCharacter (Components|GetOwner)))
  (Variables|Default|SetBoneBladeCharacter _asbp_bone_blade_mutant_character))

(event EventTick
  (params (DeltaSeconds :type Float%20%28single-precision%29)))

(fn GetFireLocation
  (if (Variables|Default|GetisRight)
    (Variables|Default|SetFireLocation (Transformation|GetSocketLocation (Variables|/Script/Engine.Character|GetMesh (Variables|Default|GetBoneBladeCharacter)) "R_BoneBladeSocket"))
    (Variables|Default|SetisRight false)
    (else
      (Variables|Default|SetFireLocation (Transformation|GetSocketLocation (Variables|/Script/Engine.Character|GetMesh (Variables|Default|GetBoneBladeCharacter)) "L_BoneBladeSocket"))
      (Variables|Default|SetisRight true))))