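; Playable Bone Blade mutant character with three input abilities: a bone projectile fired through its component, a print-only Sharpen Bones, and a charged area attack.
; Holding Ability3 slows movement while a looping timer grows capped power and radius.
; Release expands a timeline-scaled debug-drawn sphere that gathers overlapping BaseEnemy actors, only printing their names.
; Melee and sheath montage events are unwired stubs, alongside a combo-window validity macro.
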(event Custom|BoneAOE
  (bind _overlapping_actors (Variables|Default|GetOverlapping%20Actors))
  (if (not (Variables|Default|GetAOETriggered))
    (Variables|Default|SetAOETriggered true)
    (bind _returnvalue (AddComponent|AddSphereComponent false))
    (bind _newtrack_0 (Timeline|SphereTrace PlayFromStart)
      (:Update
        (Transformation|SetWorldScale3D _returnvalue (Math|Vector|Lerp(Vector) "0, 0, 0" (Variables|Default|GetAOE%20Radius) _newtrack_0))
        (Rendering|Debug|DrawDebugSphere (Transformation|GetActorLocation) (Components|Sphere|GetScaledSphereRadius _returnvalue) 12 "(R=0.030518,G=1.000000,B=0.000000,A=1.000000)" 0.1 0.5)
        (for _array_element (Collision|GetOverlappingActors _returnvalue "/Script/Malignant.BaseEnemy" :!class /Script/Engine.PrimitiveComponent)
          (Utilities|Set|Add (Variables|Default|GetOverlapping%20Actors) _array_element)))
      (:Finished
        (Components|DestroyComponent _returnvalue)
        (if (Utilities|Set|IsEmpty _overlapping_actors)
          _
          (else
            (bind _result (Utilities|Set|ToArray _overlapping_actors))
            (for _array_element_2 _result
              (Development|PrintString (Utilities|GetDisplayName _array_element_2)))
            (Utilities|Set|Clear (Variables|Default|GetOverlapping%20Actors))))
        (Variables|Default|SetAOE%20Radius "0, 0, 0")
        (Variables|Default|SetAOETriggered false)
        (Development|PrintString "Reset")))))

(event Custom|lightAttackEvent
  ;[1 1 1] montage events sample
)

(event Custom|heavyAttackEvent
  ;[1 1 1] montage events sample
)

(event Custom|sheathBladesEvent
  ;[1 1 1] montage events sample
)

(event Custom|spinAttackEvent
  ;[1 1 1] montage events sample
)

(event Custom|unsheathBladesEvent
  ;[1 1 1] montage events sample
)

(event EventBeginPlay)

(event Collision|EventActorBeginOverlap
  (params (OtherActor :type Actor%20Object%20Reference)))

(event EventTick
  (params (DeltaSeconds :type Float%20%28single-precision%29)))

(event Input|ActionEvents|InputActionAbility1
  (params (Key :type Key%20Structure :default "None"))
  (:Pressed
    (Default|FireBone (Variables|Default|GetBP_BoneProjectileComponent))))

(event Input|ActionEvents|InputActionAbility2
  (params (Key :type Key%20Structure :default "None"))
  (:Pressed
    (CallFunction|SharpenBones)))

(event Input|ActionEvents|InputActionAbility3
  (params (Key :type Key%20Structure :default "None"))
  (:Pressed
    (if (not (Variables|Default|GetAOETriggered))
      (Variables|/Script/Engine.CharacterMovementComponent|SetMaxWalkSpeed (Variables|Character|GetCharacterMovement) 5e+01)
      (bind _returnvalue (Utilities|Time|SetTimerbyFunctionName 0 "AddCharge" 0.2 true))
      (Variables|Default|SetAOEChargeHandle _returnvalue)))
  (:Released
    (Variables|/Script/Engine.CharacterMovementComponent|SetMaxWalkSpeed (Variables|Character|GetCharacterMovement) 6e+02)
    (Utilities|Time|ClearandInvalidateTimerbyHandle (Variables|Default|GetAOEChargeHandle))
    (if (> (Variables|Default|GetAOEPower) 0)
      (Variables|Default|SetAOEPower 0)
      (CallFunction|BoneAOE))))

(fn ConstructionScript)

(fn SharpenBones
  (Development|PrintString "*Shing *Shing  Damn boy now you doing hella damage "))

(fn AddCharge
  (if (< (Variables|Default|GetAOEPower) 10)
    (Math|Integer|IncrementInt (Variables|Default|GetAOEPower)
      (:%20%20
        (bind _output_get (Variables|Default|SetAOE%20Radius (+ (Variables|Default|GetAOE%20Radius) "2.000000,2.000000,2.000000")))
        (Development|PrintString (Utilities|String|ToString(Vector) _output_get))))))